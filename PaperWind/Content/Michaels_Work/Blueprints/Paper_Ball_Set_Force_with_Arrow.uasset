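; Player-controlled paper ball pawn that is launched by clicking and releasing the mouse, with an arrow actor spawned while held.
; While a Gate is open, Tick derives direction and strength from the cursor's line-plane intersection, and release fires a velocity-change impulse through a DoOnce.
; Launches are capped at two until the sphere registers a hit.
; Axis inputs add forward/back force and yaw the controller; Pause opens a menu.
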(event OnComponentHit(Sphere)
  (params (HitComponent :type Primitive%20Component%20Object%20Reference) (OtherActor :type Actor%20Object%20Reference) (OtherComp :type Primitive%20Component%20Object%20Reference) (NormalImpulse :type Vector :default "0, 0, 0") (Hit :type Hit%20Result%20Structure%20%28by%20ref%29))
  ;[1 1 1] 3 Clicks until stop
  (Variables|Default|SetClicks 0))

(event Custom|Spawn%20arrow
  ;[1 1 1] Spawn/Destroy Arrow
  (bind _returnvalue (Game|SpawnActorfromClass "/Game/Michaels_Work/Blueprints/BP_Arrow.BP_Arrow_C" (Transformation|GetActorTransform) "Undefined" 0 0))
  (Variables|Default|SetArrow_BP _returnvalue))

(event Custom|Destroy%20Arrow
  ;[1 1 1] Spawn/Destroy Arrow
  (Actor|DestroyActor (Variables|Default|GetArrow_BP)))

(event EventBeginPlay
  (bind _returnvalue (Game|GetPlayerController 0))
  ;[1 1 1] Show Mouse Cursor
  (Variables|/Script/Engine.PlayerController|SetbShowMouseCursor _returnvalue true)
  (Variables|/Script/Engine.PlayerController|SetbEnableClickEvents _returnvalue true)
  (Game|Player|SetViewTargetwithBlend _returnvalue self 0.0 "VTBlend_Linear" 0.0 false))

(event EventTick
  (params (DeltaSeconds :type Float%20%28single-precision%29))
  (bind _returnvalue (Game|GetPlayerCameraManager 0))
  (bind _returnvalue_2 (Transformation|GetActorLocation))
  (bind _returnvalue_3 (Game|GetPlayerController 0))
  (bind _returnvalue_4 (Transformation|GetActorLocation))
  (bind _returnvalue_5 (Camera|GetCameraLocation _returnvalue))
  (bind (_worldlocation _worlddirection) (Game|Player|ConvertMouseLocationToWorldSpace _returnvalue_3))
  (bind _returnvalue_6 (* _worlddirection 5e+03))
  (bind _returnvalue_7 (+ _worldlocation _returnvalue_6))
  (bind _intersection (Class|KismetMathLibrary|LinePlaneIntersectionOriginNormal _returnvalue_5 _returnvalue_7 _returnvalue_4 _returnvalue_7))
  ;[0.2744 1 0.3854] Ball Move Mechanic
  (Utilities|FlowControl|Gate true
    (:Exit
      ;;[1 1 1] Set force and direction based on mouse point
      (Variables|Default|SetDirection (Math|Vector|GetUnitDirection(Vector) _returnvalue_2 _intersection))
      (Variables|Default|SetMagnitude (* (Math|Vector|VectorLength (- _returnvalue_2 _intersection)) 12.0))
      (Utilities|FlowControl|Delay 0.5)
      ;;[1 1 1] Add Force
      (Utilities|FlowControl|DoOnce false) ; enters at Reset
    )))

(event Input|ActionEvents|InputActionPause
  (params (Key :type Key%20Structure :default "None"))
  (bind _returnvalue (Game|GetPlayerController 0))
  (:Pressed
    (Utilities|IsValid (Variables|Default|GetPauseMenuReference)
      (:Is%20Valid
        _)
      (:Is%20Not%20Valid
        (bind _returnvalue_2 (UserInterface|CreateWidget "/Game/Lachlans_Work/3D_Menu/Widgets/PauseMenu.PauseMenu_C"))
        (Variables|Default|SetPauseMenuReference _returnvalue_2)))
    (Variables|/Script/Engine.PlayerController|SetbShowMouseCursor _returnvalue true)
    (Input|SetInputModeUIOnly _returnvalue (Variables|Default|GetPauseMenuReference) "DoNotLock")
    (UserInterface|Viewport|AddtoViewport (Variables|Default|GetPauseMenuReference) 0)
    (Game|SetGamePaused true)))

(event Input|AxisEvents|InputAxisMoveForward
  (params (AxisValue :type Float%20%28single-precision%29))
  ;[1 1 1] W and S movement
  (Physics|AddForce (Variables|Default|GetSphere) (* (Math|Vector|MakeVector AxisValue 0.0 0.0) 8e+04) "None" false))

(event Input|AxisEvents|InputAxisMoveRight
  (params (AxisValue :type Float%20%28single-precision%29))
  ;[1 1 1] Move Camera
  (Pawn|Input|AddControllerYawInput AxisValue)
  (Pawn|SetControlRotation (Game|GetPlayerController 0) (Math|Rotator|MakeRotator 0.0 0.0 (.yaw (Pawn|GetControlRotation :!class /Script/Engine.Pawn)))))

(event Input|MouseEvents|LeftMouseButton
  (params (Key :type Key%20Structure :default "None"))
  (bind _returnvalue (Game|GetPlayerCameraManager 0))
  (bind _returnvalue_2 (Transformation|GetActorLocation))
  (bind _returnvalue_3 (Game|GetPlayerController 0))
  (bind _returnvalue_4 (Transformation|GetActorLocation))
  (bind _returnvalue_5 (Camera|GetCameraLocation _returnvalue))
  (bind (_worldlocation _worlddirection) (Game|Player|ConvertMouseLocationToWorldSpace _returnvalue_3))
  (bind _returnvalue_6 (* _worlddirection 5e+03))
  (bind _returnvalue_7 (+ _worldlocation _returnvalue_6))
  (bind _intersection (Class|KismetMathLibrary|LinePlaneIntersectionOriginNormal _returnvalue_5 _returnvalue_7 _returnvalue_4 _returnvalue_7))
  ;[1 1 1] 3 Clicks until stop
  (:Pressed
    (if (< (Variables|Default|GetClicks) 2)
      (Variables|Default|SetCan%20Release true)
      ;[0.2744 1 0.3854] Ball Move Mechanic
      (CallFunction|SpawnArrow)
      (Math|Integer|IncrementInt (Variables|Default|GetClicks)
        (:%20%20
          (Utilities|FlowControl|Gate true) ; enters at Open
        ))))
  (:Released
    (if (Variables|Default|GetCan%20Release)
      (Variables|Default|SetCan%20Release false)
      (CallFunction|DestroyArrow)
      ;;[1 1 1] Add Force
      (Utilities|FlowControl|DoOnce false
        (:Completed
          (Physics|AddImpulse (Variables|Default|GetSphere) (* (Variables|Default|GetDirection) (Variables|Default|GetMagnitude)) "None" true)
          (Utilities|FlowControl|Gate true) ; enters at Close
        )))))

(fn ConstructionScript)

(fn ReturnNode)

(fn ReturnCursortoScreen)