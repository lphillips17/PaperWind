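; Arrow indicator actor that stays on the player pawn and points toward the mouse cursor.
; Every Tick it moves to the pawn and rotates toward where a camera-to-cursor line intersects a plane through the arrow.
; That plane's normal is the deprojected cursor's far point, used as a vector, rather than a fixed axis.
; The Arrow component scales uniformly with the distance to that intersection.
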(event EventBeginPlay)

(event Collision|EventActorBeginOverlap
  (params (OtherActor :type Actor%20Object%20Reference)))

(event EventTick
  (params (DeltaSeconds :type Float%20%28single-precision%29))
  (bind _returnvalue (Game|GetPlayerCameraManager 0))
  (bind _returnvalue_2 (Game|GetPlayerController 0))
  (bind _returnvalue_3 (Transformation|GetActorLocation))
  (bind _returnvalue_4 (Transformation|GetActorLocation))
  (bind _returnvalue_5 (Camera|GetCameraLocation _returnvalue))
  (bind (_worldlocation _worlddirection) (Game|Player|ConvertMouseLocationToWorldSpace _returnvalue_2))
  (bind _returnvalue_6 (* _worlddirection 5e+03))
  (bind _returnvalue_7 (+ _worldlocation _returnvalue_6))
  (bind _intersection (Class|KismetMathLibrary|LinePlaneIntersectionOriginNormal _returnvalue_5 _returnvalue_7 _returnvalue_3 _returnvalue_7))
  (bind _returnvalue_8 (Math|Vector|Distance(Vector) _returnvalue_4 _intersection))
  (bind _returnvalue_9 (* _returnvalue_8 0.05))
  (Transformation|SetActorLocation (Transformation|GetActorLocation (Game|Player|GetPlayerPawn 0)) false false)
  (Transformation|SetActorRotation (Math|Rotator|FindLookatRotation _returnvalue_4 _intersection))
  (Transformation|SetRelativeScale3D (Variables|Default|GetArrow) (Math|Vector|MakeVector _returnvalue_9 _returnvalue_9 _returnvalue_9)))

(fn ConstructionScript)