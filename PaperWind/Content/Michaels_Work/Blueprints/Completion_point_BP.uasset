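; Level goal trigger that ends the game in a win when the paper ball reaches its box.
; A one-shot box overlap checks for the paper ball, then calls HasWon on Main_GM, shows the win widget and spawns confetti at hardcoded world locations.
; After a short delay it opens the main menu level.
; The one-shot gate precedes the ball check, so any first overlapping actor uses it up.
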(event OnComponentBeginOverlap(Box)
  (params (OverlappedComponent :type Primitive%20Component%20Object%20Reference) (OtherActor :type Actor%20Object%20Reference) (OtherComp :type Primitive%20Component%20Object%20Reference) (OtherBodyIndex :type Integer) (bFromSweep :type Boolean) (SweepResult :type Hit%20Result%20Structure%20%28by%20ref%29))
  (Utilities|FlowControl|DoOnce false
    (:Completed
      (bind _aspaper_ball_set_force_with_arrow (Utilities|Casting|CastToPaper_Ball_Set_Force_with_Arrow OtherActor))
      (bind _asmain_gm (Utilities|Casting|CastToMain_GM (Game|GetGameMode)))
      (Default|HasWon _asmain_gm)
      (bind _returnvalue (UserInterface|CreateWidget "/Game/Michaels_Work/Widgets/You_Win_Widget.You_Win_Widget_C"))
      (UserInterface|Viewport|AddtoViewport _returnvalue 0)
      (Effects|SpawnEmitteratLocation "/Game/Michaels_Work/Materials/Emitters/P_Confetti.P_Confetti" "550.000000,-3320.000000,140.000000")
      (Effects|SpawnEmitteratLocation "/Game/Michaels_Work/Materials/Emitters/P_Confetti.P_Confetti" "650.000000,-3320.000000,140.000000")
      (Utilities|FlowControl|Delay 4.0)
      (Game|OpenLevel(byName) "Main_Menu_Level"))))

(event EventBeginPlay)

(event EventTick
  (params (DeltaSeconds :type Float%20%28single-precision%29)))

(fn ConstructionScript)