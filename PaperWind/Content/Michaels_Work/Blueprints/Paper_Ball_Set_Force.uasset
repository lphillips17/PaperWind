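; Player-controlled paper ball that is launched toward the mouse cursor with a physics impulse.
; Left click opens a Tick gate that draws a debug aim arrow to the cursor ray's plane intersection, updating direction and distance-scaled magnitude.
; After a short delay, a DoOnce node leads to the velocity-change impulse on the Sphere and closes the gate.
; Movement axes also push the sphere along world X and yaw the controller.
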(event EventBeginPlay
  (bind _returnvalue (Game|GetPlayerController 0))
  (Variables|/Script/Engine.PlayerController|SetbShowMouseCursor _returnvalue true)
  (Variables|/Script/Engine.PlayerController|SetbEnableClickEvents _returnvalue true)
  (Game|Player|SetViewTargetwithBlend _returnvalue self 0.0 "VTBlend_Linear" 0.0 false))

(event Collision|EventActorBeginOverlap
  (params (OtherActor :type Actor%20Object%20Reference)))

(event EventTick
  (params (DeltaSeconds :type Float%20%28single-precision%29))
  (bind _returnvalue (Game|GetPlayerCameraManager 0))
  (bind _returnvalue_2 (Transformation|GetActorLocation))
  (bind _returnvalue_3 (Transformation|GetActorLocation))
  (bind _returnvalue_4 (Game|GetPlayerController 0))
  (bind _returnvalue_5 (Camera|GetCameraLocation _returnvalue))
  (bind (_worldlocation _worlddirection) (Game|Player|ConvertMouseLocationToWorldSpace _returnvalue_4))
  (bind _returnvalue_6 (* _worlddirection 5e+03))
  (bind _returnvalue_7 (+ _worldlocation _returnvalue_6))
  (bind _intersection (Class|KismetMathLibrary|LinePlaneIntersectionOriginNormal _returnvalue_5 _returnvalue_7 _returnvalue_3 _returnvalue_7))
  (Utilities|FlowControl|Gate true :!label _label
    (:Exit
      (Rendering|Debug|DrawDebugArrow _returnvalue_2 _intersection 2e+01 "(R=0.063332,G=1.000000,B=0.000000,A=1.000000)" 0.0 2.0)
      (Variables|Default|SetDirection (Math|Vector|GetUnitDirection(Vector) _returnvalue_2 _intersection))
      (Variables|Default|SetMagnitude (* (Math|Vector|VectorLength (- _returnvalue_2 _intersection)) 12.0))
      (Utilities|FlowControl|Delay 0.75)
      (Utilities|FlowControl|DoOnce false ; enters at Reset
        (:Completed
          (Physics|AddImpulse (Variables|Default|GetSphere) (* (Variables|Default|GetDirection) (Variables|Default|GetMagnitude)) "None" true)
          (goto _label Close))))))

(event Input|AxisEvents|InputAxisMoveForward
  (params (AxisValue :type Float%20%28single-precision%29))
  (Physics|AddForce (Variables|Default|GetSphere) (* (Math|Vector|MakeVector AxisValue 0.0 0.0) 8e+04) "None" false))

(event Input|AxisEvents|InputAxisMoveRight
  (params (AxisValue :type Float%20%28single-precision%29))
  (Pawn|Input|AddControllerYawInput AxisValue)
  (Pawn|SetControlRotation (Game|GetPlayerController 0) (Math|Rotator|MakeRotator 0.0 0.0 (.yaw (Pawn|GetControlRotation :!class /Script/Engine.Pawn)))))

(event Input|MouseEvents|LeftMouseButton
  (params (Key :type Key%20Structure :default "None"))
  (bind _returnvalue (Game|GetPlayerCameraManager 0))
  (bind _returnvalue_2 (Transformation|GetActorLocation))
  (bind _returnvalue_3 (Transformation|GetActorLocation))
  (bind _returnvalue_4 (Game|GetPlayerController 0))
  (bind _returnvalue_5 (Camera|GetCameraLocation _returnvalue))
  (bind (_worldlocation _worlddirection) (Game|Player|ConvertMouseLocationToWorldSpace _returnvalue_4))
  (bind _returnvalue_6 (* _worlddirection 5e+03))
  (bind _returnvalue_7 (+ _worldlocation _returnvalue_6))
  (bind _intersection (Class|KismetMathLibrary|LinePlaneIntersectionOriginNormal _returnvalue_5 _returnvalue_7 _returnvalue_3 _returnvalue_7))
  (:Pressed
    (Utilities|FlowControl|Gate true) ; enters at Open
  ))

(fn ConstructionScript)

(fn ReturnNode)

(fn ReturnCursortoScreen)