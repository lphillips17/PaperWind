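; Paper ball actor prototype that builds a launch-style Force vector from mouse drags and visualizes it, without applying it.
; Pressing the left mouse button zeroes Force and opens a Gate on Tick; releasing closes it.
; While open, each frame's mouse delta is projected onto the world X axis, scaled and accumulated into Force, drawn as a debug arrow from the actor.
; The cursor-return function and construction script are empty.
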(event Collision|EventActorBeginOverlap
  (params (OtherActor :type Actor%20Object%20Reference)))

(event EventTick
  (params (DeltaSeconds :type Float%20%28single-precision%29))
  (bind _returnvalue (Game|GetPlayerController 0))
  (bind _returnvalue_2 (Transformation|GetActorLocation))
  (bind (_deltax _deltay) (Class|PlayerController|GetInputMouseDelta _returnvalue))
  (bind _returnvalue_3 (Math|Vector2D|MakeVector2D _deltax _deltay))
  (bind (_outdir _outlength) (Class|KismetMathLibrary|ToDirectionandLength2D _returnvalue_3))
  (Utilities|FlowControl|Gate true
    (:Exit
      (bind _output_get (Variables|Default|SetForce (+ (Variables|Default|GetForce) (* (Math|Vector|ProjectVectorontoVector (Math|Conversions|ToVector(Vector2D) _outdir) "1.000000, 0, 0") (* _outlength 5e+01)))))
      (Rendering|Debug|DrawDebugArrow _returnvalue_2 (+ _output_get _returnvalue_2) 2e+02 "(R=0.000000,G=1.000000,B=0.089374,A=1.000000)" 0.0 3.0))))

(event Input|MouseEvents|LeftMouseButton
  (params (Key :type Key%20Structure :default "None"))
  (bind _returnvalue (Game|GetPlayerController 0))
  (bind _returnvalue_2 (Transformation|GetActorLocation))
  (bind (_deltax _deltay) (Class|PlayerController|GetInputMouseDelta _returnvalue))
  (bind _returnvalue_3 (Math|Vector2D|MakeVector2D _deltax _deltay))
  (bind (_outdir _outlength) (Class|KismetMathLibrary|ToDirectionandLength2D _returnvalue_3))
  (:Pressed
    (Variables|Default|SetForce "0, 0, 0")
    (Utilities|FlowControl|Gate true) ; enters at Open
  )
  (:Released
    (Utilities|FlowControl|Gate true) ; enters at Close
  ))

(fn ConstructionScript)

(fn ReturnNode)

(fn ReturnCursortoScreen)